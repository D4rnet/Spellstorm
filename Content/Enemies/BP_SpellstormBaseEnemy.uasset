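; BP_SpellstormBaseEnemy is a base enemy with a melee attack, stat-driven damage intake and death handling.
; A collision sphere, sized from an ACStatSystem stat, tracks the overlapping actor to damage.
; Attack plays a montage, then applies fixed damage to that actor and signals attack end.
; Incoming damage modifies a stat; on death it animates, stops AI logic, disables collision and expires shortly after.
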(event OnComponentBeginOverlap(AttackCollisionSphere)
  (params (OverlappedComponent :type Primitive%20Component%20Object%20Reference) (OtherActor :type Actor%20Object%20Reference) (OtherComp :type Primitive%20Component%20Object%20Reference) (OtherBodyIndex :type Integer) (bFromSweep :type Boolean) (SweepResult :type Hit%20Result%20Structure%20%28by%20ref%29))
  (Variables|Default|SetPlayerToDamage OtherActor))

(event OnComponentEndOverlap(AttackCollisionSphere)
  (params (OverlappedComponent :type Primitive%20Component%20Object%20Reference) (OtherActor :type Actor%20Object%20Reference) (OtherComp :type Primitive%20Component%20Object%20Reference) (OtherBodyIndex :type Integer))
  (Variables|Default|SetPlayerToDamage 0))

(event Custom|Attack
  (Animation|Montage|PlayMontage (Variables|Character|GetMesh) "/Game/Meshes/BattleWizardPolyart/Animations/AM_Attack04Anim.AM_Attack04Anim" 2.0
    (:OnCompleted
      (Game|Damage|ApplyDamage (Variables|Default|GetPlayerToDamage) 1e+01 0 self)
      (Default|CallOnAttackEnd))))

(event EventBeginPlay
  (EventDispatchers|BindEventtoOnDeath (Variables|Default|GetAC_StatSystem) (EventDispatchers|CreateEvent :!event OnDeath)))

(event Game|Damage|EventAnyDamage
  (params (Damage :type Float%20%28single-precision%29) (DamageType :type Damage%20Type%20Object%20Reference) (InstigatedBy :type Controller%20Object%20Reference) (DamageCauser :type Actor%20Object%20Reference))
  (Default|ModifyStat (Variables|Default|GetAC_StatSystem) "NewEnumerator1" "NewEnumerator3" "NewEnumerator3" Damage))

(fn ConstructionScript
  (Components|Sphere|SetSphereRadius (Variables|Default|GetAttackCollisionSphere) (Default|GetStatValue (Variables|Default|GetAC_StatSystem) "NewEnumerator3" "NewEnumerator5") true))

(fn OnDeath
  (bind _self self)
  (bind _returnvalue (AI|GetAIController _self))
  (Animation|PlayAnimMontage "/Game/Meshes/BattleWizardPolyart/Animations/AM_DieAnim.AM_DieAnim" 1.0 "None")
  (AI|ClearFocus _returnvalue)
  (AI|Logic|StopLogic (Variables|/Script/AIModule.AIController|GetBrainComponent _returnvalue) "")
  (Collision|SetActorEnableCollision false)
  (Variables|Actor|SetbCanBeDamaged false)
  (Actor|SetLifeSpan 2.0))