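; BP_MeshesSpawn is a landscape scattering actor that places grass and tree mesh instances within a box volume.
; SpawnMeshes picks each mesh variant, sizes the Container box, then adds instances with random yaw at trace hits, ignoring hits on itself.
; LineFunc supplies those hits by tracing downward from raised random points in the box against configured object types.
; The construction script's SpawnMeshes call is disconnected, so nothing in this graph runs it.
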(event EventBeginPlay)

(event Collision|EventActorBeginOverlap
  (params (OtherActor :type Actor%20Object%20Reference)))

(event EventTick
  (params (DeltaSeconds :type Float%20%28single-precision%29)))

(fn ConstructionScript)

(fn SpawnMeshes
  (bind _tree (Variables|Default|GetTree))
  (bind _grass (Variables|Default|GetGrass))
  (bind _scale (Variables|Default|GetScale))
  (Utilities|FlowControl|Sequence
    (:then_0
      (switch int (Variables|Grass|GetVariation%20Grass)
        (:0
          (Components|StaticMesh|SetStaticMesh _grass (Variables|Grass|GetGrass%20Mesh%201)))
        (:1
          (Components|StaticMesh|SetStaticMesh _grass (Variables|Grass|GetGrass%20Mesh%202)))))
    (:then_1
      (Utilities|FlowControl|Sequence
        (:then_0
          (switch int (Variables|Tree|GetVariation%20Tree)
            (:0
              (Components|StaticMesh|SetStaticMesh _tree (Variables|Tree|GetTree%20Mesh%201)))
            (:1
              (Components|StaticMesh|SetStaticMesh _tree (Variables|Tree|GetTree%20Mesh%202)))))
        (:then_1
          (if (Utilities|Operators|EqualEqual :A (Variables|Default|GetScale%20Container))
            (Variables|Default|SetScale%20Container (Math|Vector|MakeVector _scale _scale _scale)))
          (Components|Box|SetBoxExtent (Variables|Default|GetContainer) (Variables|Default|GetScale%20Container) false)
          (for _index (range 0 (- (Variables|Grass|GetCounter%20Grass) 1))
            (bind (_returnvalue _outhit) (Utilities|LineFunc))
            (if _returnvalue
              (if (!= (.HitActor (Collision|BreakHitResult _outhit)) self)
                (Components|InstancedStaticMesh|AddInstance (Variables|Default|GetGrass) (Math|Transform|MakeTransform (.ImpactPoint (Collision|BreakHitResult _outhit)) (Math|Rotator|MakeRotator 0.0 0.0 (Math|Random|RandomFloatinRange 0.0 (Variables|Grass|GetMaxRotation%20Grass))) (Math|Conversions|ToVector(Float) (Variables|Grass|GetGrass%20MeshScale))) true))))
          (for _index_2 (range 0 (- (Variables|Tree|GetCounter%20Tree) 1))
            (bind (_returnvalue_2 _outhit_2) (Utilities|LineFunc))
            (if _returnvalue_2
              (if (!= (.HitActor (Collision|BreakHitResult _outhit_2)) self)
                (Components|InstancedStaticMesh|AddInstance (Variables|Default|GetTree) (Math|Transform|MakeTransform (.ImpactPoint (Collision|BreakHitResult _outhit_2)) (Math|Rotator|MakeRotator 0.0 0.0 (Math|Random|RandomFloatinRange 0.0 (Variables|Tree|GetMaxRotation%20Tree))) (Math|Conversions|ToVector(Float) (Variables|Tree|GetTree%20Mesh%20Scale))) true)))))))))