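; Enemy spawner that keeps adding Enem actors around player 0 on a looping half-second timer.
; Each tick queries a random reachable navmesh point around the player and requires it to lie beyond a minimum distance.
; A failed check retries by immediate, unbounded recursion.
; The spawn location comes from a separate random query, so it is not necessarily the point that passed the check.
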(event Custom|Try%20Spawn%20Enemy
  (bind _returnvalue (Game|Player|GetPlayerPawn 0))
  (bind _returnvalue_2 (Transformation|GetActorLocation _returnvalue))
  (bind _randomlocation (AI|Navigation|GetRandomReachablePointinRadius _returnvalue_2 6e+03 0 0))
  (if (> (Math|Vector|VectorLength (- _returnvalue_2 _randomlocation)) 3e+03)
    (Game|SpawnActorfromClass "/Game/Landscape/enem.enem_C" (Math|Transform|MakeTransform _randomlocation "0, 0, 0" "1.000000,1.000000,1.000000") "Undefined" "MultiplyWithRoot" 0 0)
    (else
      (CallFunction|TrySpawnEnemy))))

(event EventBeginPlay
  (Utilities|Time|SetTimerbyEvent (delegate Custom|Try%20Spawn%20Enemy) 0.5 true))

(fn ConstructionScript)