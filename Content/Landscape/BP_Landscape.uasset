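; BP_Landscape streams a chunked landscape around the player pawn, with grass and tree meshes on each chunk.
; Each Tick converts the pawn location to grid coordinates and fills missing cells within Distance with a configured BP_Chunk and BP_MeshesSpawn pair.
; The Generated set and AllChunksArray track spawned cells.
; When the player's cell matches the previous one, it destroys tracked pairs on the ring one cell beyond Distance.
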(event EventTick
  (params (DeltaSeconds :type Float%20%28single-precision%29))
  (bind _current (Variables|Default|GetCurrent))
  (bind _current_2 (Variables|Default|GetCurrent))
  (bind _scale (Variables|Default|GetScale))
  (bind _current_3 (Variables|Default|GetCurrent))
  (bind _current_4 (Variables|Default|GetCurrent))
  (|CalculateChunkPos)
  (bind _index (Utilities|NewMacro)
    (:LoopBody
      (Variables|Default|SetX _index)
      (bind _index_2 (Utilities|NewMacro)
        (:LoopBody
          (Variables|Default|SetY _index_2)
          (Variables|Default|SetVisible (Utilities|Struct|MakeSTRK_ChunkPosition (+ (.x _current_2) (Variables|Default|GetX)) (+ (.y _current_2) (Variables|Default|GetY))))
          (if (not (Utilities|Set|Contains (Variables|Default|GetGenerated) (Variables|Default|GetVisible)))
            (bind _returnvalue (Game|SpawnActorfromClass "/Game/Landscape/BP_Chunk.BP_Chunk_C" (Math|Transform|MakeTransform (Math|Vector|MakeVector (* (.x (Variables|Default|GetVisible)) _scale) (* _scale (.y (Variables|Default|GetVisible))) 0.0) "0, 0, 0" "1.000000,1.000000,1.000000") "Undefined" "MultiplyWithRoot" 0 0))
            (bind _output_get (Variables|Default|SetChunk _returnvalue))
            (CallFunction|SetChunkParametrs _output_get)
            (Default|Generate (Variables|Default|GetChunk))
            (bind _returnvalue_2 (CallFunction|SpawnMeshSpawn))
            (bind _output_get_2 (Variables|GrassSpawn|SetSpawnMeshes _returnvalue_2))
            (CallFunction|SetMeshSpawnParametrs _output_get_2 (Variables|GrassSpawn|GetCounter%20Grass) (Variables|GrassSpawn|GetMax%20Rotation%20Grass) (Variables|GrassSpawn|GetGrass%20Variation) (Variables|GrassSpawn|GetGrass1) (Variables|GrassSpawn|GetGrass2) (Variables|GrassSpawn|GetGrass%20Mesh%20Scale) (Variables|GrassSpawn|GetCounter%20Tree) (Variables|GrassSpawn|GetMax%20Rotation%20Tree) (Variables|GrassSpawn|GetVariation%20Spawn%20Tree) (Variables|GrassSpawn|GetTree%20Mesh%201) (Variables|GrassSpawn|GetTree%20Mesh%202) (Variables|GrassSpawn|GetTree%20Scale%20Spawn))
            (Default|SpawnMeshes (Variables|GrassSpawn|GetSpawnMeshes))
            (Utilities|Set|Add (Variables|Default|GetGenerated) (Variables|Default|GetVisible))
            (Utilities|Array|Add (Variables|Default|GetAllChunksArray) (Utilities|Struct|MakeSTRK_ChunksCoordinates (Variables|Default|GetVisible) (Variables|Default|GetChunk) (Variables|GrassSpawn|GetSpawnMeshes)))))))
    (:Completed
      (if (and (== (.x _current_3) (.x (Variables|Default|GetPrevious))) (== (.y _current_3) (.y (Variables|Default|GetPrevious))))
        (bind (_index_3 _returnvalue_3) (Utilities|NewMacro0)
          (:LoopBody
            (Variables|Default|SetXdel _index_3)
            (bind (_index_4 _returnvalue_4) (Utilities|NewMacro0)
              (:LoopBody
                (Variables|Default|SetYdel _index_4)
                (if (or _returnvalue_4 _returnvalue_3)
                  (Variables|Default|SetVisibleDeletingSTRK (Utilities|Struct|MakeSTRK_ChunkPosition (+ (Variables|Default|GetXdel) (.x _current)) (+ (.y _current) (Variables|Default|GetYdel))))
                  (if (not (Utilities|Set|Contains (Variables|Default|GetDeleting%20STRK) (Variables|Default|GetVisibleDeletingSTRK)))
                    (Utilities|Set|Add (Variables|Default|GetDeleting%20STRK) (Variables|Default|GetVisibleDeletingSTRK))
                    (bind _result (Utilities|Set|ToArray (Variables|Default|GetDeleting%20STRK)))
                    (for _array_element _result
                      (Variables|Default|SetXdelLoop (.x _array_element))
                      (Variables|Default|SetYdelLoop (.y _array_element))
                      (bind _result_2 (Utilities|Set|ToArray (Variables|Default|GetGenerated)))
                      (for _array_element_2 _result_2
                        (if (and (== (.x _array_element_2) (Variables|Default|GetXdelLoop)) (== (.y _array_element_2) (Variables|Default|GetYdelLoop)))
                          (for _array_element_3 (Variables|Default|GetAllChunksArray)
                            (if (and (== (.x (.chunkposition _array_element_3)) (Variables|Default|GetXdelLoop)) (== (.y (.chunkposition _array_element_3)) (Variables|Default|GetYdelLoop)))
                              (Actor|DestroyActor (.chunk _array_element_3))
                              (Actor|DestroyActor (.meshedspawn _array_element_3))
                              (Utilities|Array|RemoveItem (Variables|Default|GetAllChunksArray) (Utilities|Struct|MakeSTRK_ChunksCoordinates (Utilities|Struct|MakeSTRK_ChunkPosition (Variables|Default|GetXdelLoop) (Variables|Default|GetYdelLoop)) (.chunk _array_element_3) (.meshedspawn _array_element_3)))
                              (Utilities|Set|Remove (Variables|Default|GetDeleting%20STRK) (Utilities|Struct|MakeSTRK_ChunkPosition (Variables|Default|GetXdelLoop) (Variables|Default|GetYdelLoop)))
                              (Utilities|Set|Remove (Variables|Default|GetGenerated) (Utilities|Struct|MakeSTRK_ChunkPosition (Variables|Default|GetXdelLoop) (Variables|Default|GetYdelLoop)))))
                          (else
                            (Utilities|Set|Remove (Variables|Default|GetDeleting%20STRK) (Utilities|Struct|MakeSTRK_ChunkPosition (Variables|Default|GetXdelLoop) (Variables|Default|GetYdelLoop)))))))))))))
        (else
          (Variables|Default|SetPrevious (Utilities|Struct|MakeSTRK_ChunkPosition (.x _current_4) (.y _current_4))))))))

(fn ConstructionScript)

(fn SetChunkParametrs
  (params (Chunk :type BP%20Chunk%20Object%20Reference))
  (Variables|/Game/Landscape/BP_Chunk.BP_Chunk_C|SetSize Chunk (Variables|Default|GetSize))
  (Variables|/Game/Landscape/BP_Chunk.BP_Chunk_C|SetVertix%20Distance Chunk (/ (Variables|Default|GetScale) (Variables|Default|GetSize)))
  (Variables|/Game/Landscape/BP_Chunk.BP_Chunk_C|SetZMultiplier Chunk (Variables|Default|GetZMultiplier))
  (Variables|/Game/Landscape/BP_Chunk.BP_Chunk_C|SetUVscale Chunk (Variables|Default|GetUVScale))
  (Variables|/Game/Landscape/BP_Chunk.BP_Chunk_C|SetMaterial Chunk (Variables|Default|GetMaterial)))

(fn SetMeshSpawnParametrs
  (params (SpawnMesh :type BP%20Meshes%20Spawn%20Object%20Reference) (CounterSpawn1 :type Integer) (MaxRotationSPawn1 :type Float%20%28double-precision%29) (VariationSpawn1 :type Integer) (Mesh1Spawn1 :type Static%20Mesh%20Object%20Reference) (Mesh2Spawn1 :type Static%20Mesh%20Object%20Reference) (MeshScaleSpawn1 :type Float%20%28double-precision%29) (CounterSpawn2 :type Integer) (MaxRotationSpawn2 :type Float%20%28double-precision%29) (VariationSpawn2 :type Integer) (Mesh1Spawn2 :type Static%20Mesh%20Object%20Reference) (Mesh2Spawn2 :type Static%20Mesh%20Object%20Reference) (MeshScaleSpawn2 :type Float%20%28double-precision%29))
  (Variables|/Game/Landscape/BP_MeshesSpawn.BP_MeshesSpawn_C|SetCounter%20Grass SpawnMesh CounterSpawn1)
  (Variables|/Game/Landscape/BP_MeshesSpawn.BP_MeshesSpawn_C|SetMaxRotation%20Grass SpawnMesh MaxRotationSPawn1)
  (Variables|/Game/Landscape/BP_MeshesSpawn.BP_MeshesSpawn_C|SetVariation%20Grass SpawnMesh VariationSpawn1)
  (Variables|/Game/Landscape/BP_MeshesSpawn.BP_MeshesSpawn_C|SetGrass%20Mesh%201 SpawnMesh Mesh1Spawn1)
  (Variables|/Game/Landscape/BP_MeshesSpawn.BP_MeshesSpawn_C|SetGrass%20Mesh%202 SpawnMesh Mesh2Spawn1)
  (Variables|/Game/Landscape/BP_MeshesSpawn.BP_MeshesSpawn_C|SetScale SpawnMesh (/ (Variables|Default|GetScale) 2.0))
  (Variables|/Game/Landscape/BP_MeshesSpawn.BP_MeshesSpawn_C|SetGrass%20MeshScale SpawnMesh MeshScaleSpawn1)
  (Variables|/Game/Landscape/BP_MeshesSpawn.BP_MeshesSpawn_C|SetCounter%20Tree SpawnMesh CounterSpawn2)
  (Variables|/Game/Landscape/BP_MeshesSpawn.BP_MeshesSpawn_C|SetMaxRotation%20Tree SpawnMesh MaxRotationSpawn2)
  (Variables|/Game/Landscape/BP_MeshesSpawn.BP_MeshesSpawn_C|SetVariation%20Tree SpawnMesh VariationSpawn2)
  (Variables|/Game/Landscape/BP_MeshesSpawn.BP_MeshesSpawn_C|SetTree%20Mesh%201 SpawnMesh Mesh1Spawn2)
  (Variables|/Game/Landscape/BP_MeshesSpawn.BP_MeshesSpawn_C|SetTree%20Mesh%202 SpawnMesh Mesh2Spawn2)
  (Variables|/Game/Landscape/BP_MeshesSpawn.BP_MeshesSpawn_C|SetTree%20Mesh%20Scale SpawnMesh MeshScaleSpawn2))

(fn SpawnMeshSpawn
  (bind _visible (Variables|Default|GetVisible))
  (bind _scale (Variables|Default|GetScale))
  (bind _returnvalue (Game|SpawnActorfromClass "/Game/Landscape/BP_MeshesSpawn.BP_MeshesSpawn_C" (Math|Transform|MakeTransform (Math|Vector|MakeVector (* (.x _visible) _scale) (* _scale (.y _visible)) 0.0) "0, 0, 0" "1.000000,1.000000,1.000000") "Undefined" "MultiplyWithRoot" 0 0))
  (return _returnvalue))