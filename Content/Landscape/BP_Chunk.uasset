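; BP_Chunk is a landscape chunk that builds a flat, centered square grid mesh with collision on a procedural mesh component.
; Generate fills vertices and UVs at separately scaled spacing, adds two triangles per cell, computes normals and tangents, then creates the section and applies the material.
; BeginPlay and the construction script are empty, and nothing in this file calls Generate.
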(event EventBeginPlay)

(fn ConstructionScript)

(fn CreateVertices
  (for _index (range 0 (Variables|Default|GetSize))
    (LocalVariables|SetX _index)
    (for _index_2 (range 0 (Variables|Default|GetSize))
      (LocalVariables|SetY _index_2)
      (Utilities|Array|Add (Variables|Default|GetVertices) (Math|Vector|MakeVector (.Xcoordinate (CallFunction|CalculateCoordinates (Variables|Default|GetVertix%20Distance) (LocalVariables|GetX) (LocalVariables|GetY))) (.Ycoordinate (CallFunction|CalculateCoordinates (Variables|Default|GetVertix%20Distance) (LocalVariables|GetX) (LocalVariables|GetY))) 0.0))
      (Utilities|Array|Add (Variables|Default|GetUV0) (Math|Vector2D|MakeVector2D (.Xcoordinate (CallFunction|CalculateCoordinates (Variables|Default|GetUVscale) (LocalVariables|GetX) (LocalVariables|GetY))) (.Ycoordinate (CallFunction|CalculateCoordinates (Variables|Default|GetUVscale) (LocalVariables|GetX) (LocalVariables|GetY))))))))

(fn CreateTriangles
  (for _index (range 0 (- (Variables|Default|GetSize) 1))
    (for _index_2 (range 0 (- (Variables|Default|GetSize) 1))
      (Utilities|Array|Add (Variables|Default|GetTriangles) (LocalVariables|GetVertex))
      (Utilities|Array|Add (Variables|Default|GetTriangles) (+ (LocalVariables|GetVertex) 1))
      (Utilities|Array|Add (Variables|Default|GetTriangles) (+ (Variables|Default|GetSize) (LocalVariables|GetVertex) 1))
      (Utilities|Array|Add (Variables|Default|GetTriangles) (+ (LocalVariables|GetVertex) 1))
      (Utilities|Array|Add (Variables|Default|GetTriangles) (+ (Variables|Default|GetSize) (LocalVariables|GetVertex) 2))
      (Utilities|Array|Add (Variables|Default|GetTriangles) (+ (Variables|Default|GetSize) (LocalVariables|GetVertex) 1))
      (Math|Integer|IncrementInt (LocalVariables|GetVertex)))
    (Math|Integer|IncrementInt (LocalVariables|GetVertex))))

(fn Generate
  (CallFunction|CreateVertices)
  (CallFunction|CreateTriangles)
  (|CalculateNodesandTangents_2_2)
  (Class|ProceduralMeshComponent|CreateMeshSectionLinearColor (Variables|Default|GetProceduralMesh) 0 (Variables|Default|GetVertices) (Variables|Default|GetTriangles) (Variables|Default|GetNormals) (Variables|Default|GetUV0) 0 0 0 0 (Variables|Default|GetTangents) true false)
  (Rendering|Material|SetMaterial (Variables|Default|GetProceduralMesh) 0 (Variables|Default|GetMaterial)))

(fn CalculateCoordinates
  (params (Distance :type Float%20%28double-precision%29) (X :type Integer) (Y :type Integer))
  (return (* (+ (/ (Variables|Default|GetSize) -2) X) Distance) (* (+ (/ (Variables|Default|GetSize) -2) Y) Distance)))