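; Spellstorm character that auto-attacks on a stat-driven timer, firing spells from its magic staff.
; Tick triggers the attack montage whenever the timer has readied it, speeding playback to match attack rate.
; BeginPlay binds to the anim blueprint's OnAttack, presumably for Shot timing.
; Shot spawns colored casting particles and a yaw fan of pooled projectiles, with count, spacing and scale from the stat system.
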(event EventBeginPlay
  (bind _asabp_spellstorm_character (Utilities|Casting|CastToABP_SpellstormCharacter (Components|SkeletalMesh|GetAnimInstance (Variables|Character|GetMesh))))
  (EventDispatchers|BindEventtoOnAttack _asabp_spellstorm_character (EventDispatchers|CreateEvent :!event Shot))
  (CallFunction|StartAttackTimer))

(event EventTick
  (params (DeltaSeconds :type Float%20%28single-precision%29))
  (CallFunction|TryAttack))

(fn ConstructionScript)

(fn StartAttackTimer
  (Utilities|Time|SetTimerbyFunctionName 0 "ReadyToAttack" (/ 1.0 (Default|GetStatValue (Variables|Default|GetAC_StatSystem) "NewEnumerator3" "NewEnumerator4"))))

(fn PlayAttackAnim
  (Animation|PlayAnimMontage (Variables|Animation|GetAttackAnimMontage) (Math|Float|Max(Float) (/ (Variables|Animation|GetAttackAnimPlayRate) (/ 1.0 (Default|GetStatValue (Variables|Default|GetAC_StatSystem) "NewEnumerator3" "NewEnumerator4"))) 1.0) "None"))

(fn Shot
  (bind _returnvalue (Transformation|GetActorRotation))
  (bind _returnvalue_2 (Effects|SpawnEmitteratLocation (Variables|VFX|GetCastingParticles) (Transformation|GetSocketLocation (Variables|Default|GetMagicStaff) "CastSocket") (Transformation|GetActorRotation) "0.600000,0.600000,0.600000"))
  (Effects|Components|ParticleSystem|SetVectorParameter _returnvalue_2 "color" (Math|Conversions|ToVector(LinearColor) (Variables|VFX|GetCastingParticlesColor)))
  (LocalVariables|SetStartAngle (/ (Default|GetSpreadAngle (Variables|Default|GetAC_StatSystem)) -2.0))
  (LocalVariables|SetProjectileSpacing (Default|GetStatValue (Variables|Default|GetAC_StatSystem) "NewEnumerator3" "NewEnumerator8"))
  (for _index (range 0 (- (Math|Float|Truncate (Default|GetStatValue (Variables|Default|GetAC_StatSystem) "NewEnumerator3" "NewEnumerator7")) 1))
    (Default|SpawnfromPool (Variables|Default|GetAC_ProjectilePool) (Math|Transform|MakeTransform (Transformation|GetSocketLocation (Variables|Default|GetMagicStaff) "CastSocket") (Math|Rotator|MakeRotator (.roll _returnvalue) (.pitch _returnvalue) (+ (.yaw _returnvalue) (+ (* _index (LocalVariables|GetProjectileSpacing)) (LocalVariables|GetStartAngle)))) (Math|Conversions|ToVector(Float) (Default|GetStatValue (Variables|Default|GetAC_StatSystem) "NewEnumerator3" "NewEnumerator9"))))))

(fn ReadytoAttack
  (Variables|Attack|SetCanAttack true))

(fn TryAttack
  (if (Variables|Attack|GetCanAttack)
    (CallFunction|StartAttackTimer)
    (CallFunction|PlayAttackAnim)
    (Variables|Attack|SetCanAttack false)))