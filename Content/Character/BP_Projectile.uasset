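; Reusable projectile actor that SetInUse switches on and off, toggling collision, visibility, tick and trail FX instead of destroying it.
; Activation launches it along the Box's forward vector and computes an end point at Range from the owner's location.
; Tick predicts overshoot, stops movement, then snaps to that point next frame and deactivates.
; Overlapping a non-owner actor prints its name and deactivates it; deactivation spawns the hit effect.
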(event Custom|SetInUse
  (params (InUse :type Boolean))
  (Variables|Default|SetInUse InUse)
  (Collision|SetActorEnableCollision InUse)
  (Rendering|SetActorHiddenInGame (not InUse))
  (Actor|Tick|SetActorTickEnabled InUse)
  (if InUse
    (Variables|/Script/Engine.MovementComponent|SetVelocity (Variables|Default|GetProjectileMovement) (* (Math|Vector|GetForwardVector (Variables|Default|GetBox)) (Variables|Default|Getspeed)))
    (bind _output_get (Variables|Default|SetStartLocation (Transformation|GetActorLocation (Components|GetOwner))))
    (Variables|Default|SetLastLocation (+ _output_get (* (Math|Vector|Normalize (Variables|/Script/Engine.MovementComponent|GetVelocity (Variables|Default|GetProjectileMovement))) (Variables|Default|GetRange))))
    (Components|Activation|Activate (Variables|Default|GetFX1) false)
    (else
      (Effects|SpawnEmitteratLocation (Variables|Default|GethitFx) (Transformation|GetActorLocation))
      (Components|Activation|Deactivate (Variables|Default|GetFX1)))))

(event EventBeginPlay
  (Collision|IgnoreActorwhenMoving (Variables|Default|GetBox) (Components|GetOwner) true))

(event Collision|EventActorBeginOverlap
  (params (OtherActor :type Actor%20Object%20Reference))
  (if (!= OtherActor (Components|GetOwner))
    (Development|PrintString (Utilities|GetDisplayName OtherActor))
    (CallFunction|SetinUse false)))

(event EventTick
  (params (DeltaSeconds :type Float%20%28single-precision%29))
  (if (Variables|Default|GetLastTick)
    (Transformation|SetActorLocation (Variables|Default|GetLastLocation) false false)
    (CallFunction|SetinUse false)
    (Variables|Default|SetLastTick false)
    (else
      (bind _output_get (Variables|Default|SetLastTick (>= (+ (* DeltaSeconds (Variables|Default|Getspeed)) (Math|Vector|Distance(Vector) (Variables|Default|GetStartLocation) (Transformation|GetActorLocation))) (Variables|Default|GetRange))))
      (if _output_get
        (Components|Movement|StopMovementImmediately (Variables|Default|GetProjectileMovement))))))

(fn ConstructionScript)