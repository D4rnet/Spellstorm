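; AC_Health is an actor component that tracks health for its owning actor.
; On BeginPlay it refills Health to MaxHealth and binds to the owner's OnTakeAnyDamage event.
; DamageHandling subtracts damage through SetHealth, which clamps the value between zero and MaxHealth.
; Getters expose current health and its fraction of the maximum; death is not handled here.
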(event EventBeginPlay
  (CallFunction|RefillHealth)
  (EventDispatchers|BindEventtoOnTakeAnyDamage (Components|GetOwner) (EventDispatchers|CreateEvent :!event DamageHandling)))

(fn RefillHealth
  (Variables|Default|SetHealth (Variables|Default|GetMaxHealth)))

(fn SetHealth
  (params (NewHealth :type Float%20%28double-precision%29))
  (Variables|Default|SetHealth (Math|Float|Clamp(Float) NewHealth 0.0 (Variables|Default|GetMaxHealth))))

(fn GetHealth
  (return (Variables|Default|GetHealth)))

(fn DamageHandling
  (params (DamagedActor :type Actor%20Object%20Reference) (Damage :type Float%20%28single-precision%29) (DamageType :type Damage%20Type%20Object%20Reference) (InstigatedBy :type Controller%20Object%20Reference) (DamageCauser :type Actor%20Object%20Reference))
  (CallFunction|SetHealth (- (Variables|Default|GetHealth) Damage)))

(fn GetHealthPercent
  (return (/ (Variables|Default|GetHealth) (Variables|Default|GetMaxHealth))))