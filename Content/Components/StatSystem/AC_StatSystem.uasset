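; RPG-style stat component that stores attributes, each owning scaled stats, with Default, Bonus and Total values.
; Modify functions clamp values and recompute Totals, with Total subtraction draining Bonus before Default.
; Attribute changes scale inherited stats, and adding to the first attribute fires OnLevelUp.
; Stat checks handle death, health capping and Exp thresholds, and push range and speed to the owner's AC_ProjectilePool.
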(event Custom|CheckProjectileSpeed
  (Default|SetProjectilesSpeed (Actor|GetComponentbyClass (Components|GetOwner) "/Game/Components/ObjectPool/AC_ProjectilePool.AC_ProjectilePool_C") (Stats|Getters|GetStatValue "NewEnumerator3" "NewEnumerator6")))

(event Custom|CheckExp
  (bind _value (Stats|Getters|GetStatValue "NewEnumerator3" "NewEnumerator1"))
  (bind _value_2 (Stats|Getters|GetStatValue "NewEnumerator3" "NewEnumerator0"))
  (if (>= _value _value_2)
    (Stats|Setters|SetStat "NewEnumerator0" "NewEnumerator0" (- _value _value_2))
    (Attributes|Funtions|ModifyAttribute "NewEnumerator0" "NewEnumerator1" "NewEnumerator0" 1.0)))

(event Custom|CheckRange
  (Default|SetProjectilesRange (Actor|GetComponentbyClass (Components|GetOwner) "/Game/Components/ObjectPool/AC_ProjectilePool.AC_ProjectilePool_C") (Stats|Getters|GetStatValue "NewEnumerator3" "NewEnumerator5")))

(event Custom|CheckHealth
  (bind _value (Stats|Getters|GetStatValue "NewEnumerator3" "NewEnumerator3"))
  (if (<= _value 0.0)
    (Default|CallOnDeath)
    (elif (> _value (Stats|Getters|GetStatValue "NewEnumerator3" "NewEnumerator2"))
      (Stats|Setters|SetStat "NewEnumerator1" "NewEnumerator3" (Stats|Getters|GetStatValue "NewEnumerator1" "NewEnumerator2"))
      (Stats|Setters|SetStat "NewEnumerator2" "NewEnumerator3" (Stats|Getters|GetStatValue "NewEnumerator2" "NewEnumerator2")))))

(fn GetAttributeRef
  (params (Attribute :type E_AttributeList%20Enum :default "NewEnumerator0"))
  (for (_array_element _array_index) (Utilities|Struct|BreakE_Attributes (Variables|Default|GetAttributes))
    (LocalVariables|SetAttributeValue _array_element)
    (LocalVariables|SetAttributeIndex _array_index)
    (if (Utilities|Enum|Equal(Enum) Attribute (Utilities|Struct|BreakE_SingleAttribute _array_element))
      (return (LocalVariables|GetAttributeValue) (LocalVariables|GetAttributeIndex)))))

(fn GetAttributeValue
  (params (Type :type E_StatType%20Enum :default "NewEnumerator0") (Attribute :type E_AttributeList%20Enum :default "NewEnumerator0"))
  (bind _value (Attributes|Getters|GetAttributeRef Attribute))
  (bind (_default _bonus _total) (Utilities|Struct|BreakE_SingleAttribute _value))
  (return (Utilities|Select :Index Type :NewEnumerator0 -1.0 :NewEnumerator1 _default :NewEnumerator2 _bonus :NewEnumerator3 _total)))

(fn ModifyAttribute
  (params (Operation :type E_Operators%20Enum :default "NewEnumerator0") (Type :type E_StatType%20Enum :default "NewEnumerator0") (Attribute :type E_AttributeList%20Enum :default "NewEnumerator0") (Value :type Float%20%28double-precision%29))
  (bind _value (Attributes|Getters|GetAttributeValue Type Attribute))
  (switch Utilities|FlowControl|Switch|SwitchonE_StatType Type
    (:NewEnumerator0
      (Development|PrintString "Warning: Modify Attribute -  
Error: Stat is Set to \"None\"")
      (return))
    (:NewEnumerator1
      _)
    (:NewEnumerator2
      _)
    (:NewEnumerator3
      (Attributes|Funtions|OperateTotalAttribute Operation Attribute Value)
      (return)))
  (LocalVariables|SetAttFloat _value)
  (LocalVariables|SetCalcFloat (Utilities|Select :Index Operation :NewEnumerator0 (+ _value Value) :NewEnumerator1 (- _value Value) :NewEnumerator2 Value))
  (Attributes|Setters|SetAttribute Type Attribute (LocalVariables|GetCalcFloat))
  (Attributes|Funtions|ScalingStats Type Operation (.Value (Attributes|Getters|GetAttributeRef Attribute)) (Math|Float|SelectFloat Value (LocalVariables|GetAttFloat) (> (LocalVariables|GetCalcFloat) 0.0)))
  (if (and (Utilities|Enum|Equal(Enum) Attribute "NewEnumerator0") (Utilities|Enum|Equal(Enum) Operation "NewEnumerator0"))
    (Attributes|Funtions|LevelUp Value)
    (return)))

(fn SetAttribute
  (params (Type :type E_StatType%20Enum :default "NewEnumerator0") (Attribute :type E_AttributeList%20Enum :default "NewEnumerator0") (Value :type Float%20%28double-precision%29))
  (bind (_value _index) (Attributes|Getters|GetAttributeRef Attribute))
  (LocalVariables|SetLocalAttribute _value)
  (LocalVariables|SetLocalIndex _index)
  (switch Utilities|FlowControl|Switch|SwitchonE_StatType Type
    (:NewEnumerator1
      (Utilities|Struct|SetmembersinE_SingleAttribute (LocalVariables|GetLocalAttribute) (Math|Float|Clamp(Float) Value 0.0 9999999.0) (Math|Float|Clamp(Float) (+ Value (Utilities|Struct|BreakE_SingleAttribute (LocalVariables|GetLocalAttribute))) (Utilities|Struct|BreakE_SingleAttribute (LocalVariables|GetLocalAttribute)) 9999999.0)))
    (:NewEnumerator2
      (Utilities|Struct|SetmembersinE_SingleAttribute (LocalVariables|GetLocalAttribute) (Math|Float|Clamp(Float) Value 0.0 9999999.0) (Math|Float|Clamp(Float) (+ Value (Utilities|Struct|BreakE_SingleAttribute (LocalVariables|GetLocalAttribute))) (Utilities|Struct|BreakE_SingleAttribute (LocalVariables|GetLocalAttribute)) 9999999.0)))
    (:NewEnumerator3
      (Development|PrintString "Warning: Set Attribute - 
Error: Can not set Total")
      (return)))
  (Utilities|Array|SetArrayElem (Utilities|Struct|BreakE_Attributes (Variables|Default|GetAttributes)) (LocalVariables|GetLocalIndex) (LocalVariables|GetLocalAttribute))
  (return))

(fn OperateTotalAttribute
  (params (Operation :type E_Operators%20Enum :default "NewEnumerator0") (Attribute :type E_AttributeList%20Enum :default "NewEnumerator0") (Value :type Float%20%28double-precision%29))
  (switch Utilities|FlowControl|Switch|SwitchonE_Operators Operation
    (:NewEnumerator0
      (Attributes|Funtions|ModifyAttribute "NewEnumerator0" "NewEnumerator1" Attribute Value)
      (return))
    (:NewEnumerator1
      (if (>= (- (Attributes|Getters|GetAttributeValue "NewEnumerator2" Attribute) Value) 0.0)
        (Attributes|Funtions|ModifyAttribute "NewEnumerator1" "NewEnumerator2" Attribute Value)
        (return)
        (else
          (bind _output_get (LocalVariables|SetStoredValue (Attributes|Getters|GetAttributeValue "NewEnumerator2" Attribute)))
          (Attributes|Funtions|ModifyAttribute "NewEnumerator1" "NewEnumerator2" Attribute _output_get)
          (Attributes|Funtions|ModifyAttribute "NewEnumerator1" "NewEnumerator1" Attribute (- Value (LocalVariables|GetStoredValue)))
          (return))))
    (:NewEnumerator2
      (Development|PrintString "Warning: Operate Total Attribute 
Unable to Set \"Total\" Value")
      (return))))

(fn GetStatValue
  (params (Type :type E_StatType%20Enum :default "NewEnumerator0") (Stat :type E_StatList%20Enum :default "NewEnumerator0"))
  (bind _statvalue (Stats|Getters|GetStatRef Stat))
  (bind (_default _bonus _total) (Utilities|Struct|BreakE_SingleStat _statvalue))
  (return (Utilities|Select :Index Type :NewEnumerator0 -1.0 :NewEnumerator1 _default :NewEnumerator2 _bonus :NewEnumerator3 _total)))

(fn GetStatRef
  (params (Stat :type E_StatList%20Enum :default "NewEnumerator0"))
  (for (_array_element _array_index) (Utilities|Struct|BreakE_Attributes (Variables|Default|GetAttributes))
    (bind _output_get (LocalVariables|SetAttValue _array_element))
    (LocalVariables|SetAttIndex _array_index)
    (for (_array_element_2 _array_index_2) (Utilities|Struct|BreakE_SingleAttribute _output_get)
      (LocalVariables|SetLocalStat _array_element_2)
      (LocalVariables|SetIndex _array_index_2)
      (if (Utilities|Enum|Equal(Enum) Stat (.Name (Utilities|Struct|BreakE_SingleStat _array_element_2)))
        (return (LocalVariables|GetAttValue) (LocalVariables|GetAttIndex) (LocalVariables|GetLocalStat) (LocalVariables|GetIndex))))))

(fn ModifyStat
  (params (Operation :type E_Operators%20Enum :default "NewEnumerator0") (Type :type E_StatType%20Enum :default "NewEnumerator0") (Stat :type E_StatList%20Enum :default "NewEnumerator0") (Value :type Float%20%28double-precision%29))
  (bind _value (Stats|Getters|GetStatValue Type Stat))
  (switch Utilities|FlowControl|Switch|SwitchonE_StatType Type
    (:NewEnumerator0
      (Development|PrintString "Warning: Modify Stat 
Error: Stat is set to \"None\"")
      (return))
    (:NewEnumerator1
      _)
    (:NewEnumerator2
      _)
    (:NewEnumerator3
      (Stats|Functions|OperateTotalStat Operation Stat Value)
      (return)))
  (Stats|Setters|SetStat Type Stat (Utilities|Select :Index Operation :NewEnumerator0 (+ _value Value) :NewEnumerator1 (- _value Value) :NewEnumerator2 Value))
  (Stats|Functions|ConditionalStats Stat)
  (return))

(fn SetStat
  (params (Type :type E_StatType%20Enum :default "NewEnumerator0") (Stat :type E_StatList%20Enum :default "NewEnumerator0") (Value :type Float%20%28double-precision%29))
  (LocalVariables|SetStatRef (.StatValue (Stats|Getters|GetStatRef Stat)))
  (switch Utilities|FlowControl|Switch|SwitchonE_StatType Type
    (:NewEnumerator1
      (Utilities|Struct|SetmembersinE_SingleStat (LocalVariables|GetStatRef) (Math|Float|Clamp(Float) Value 0.0 9999999.0) (Math|Float|Clamp(Float) (+ Value (Utilities|Struct|BreakE_SingleStat (LocalVariables|GetStatRef))) (Utilities|Struct|BreakE_SingleStat (LocalVariables|GetStatRef)) 9999999.0)))
    (:NewEnumerator2
      (Utilities|Struct|SetmembersinE_SingleStat (LocalVariables|GetStatRef) (Math|Float|Clamp(Float) Value 0.0 9999999.0) (Math|Float|Clamp(Float) (+ Value (Utilities|Struct|BreakE_SingleStat (LocalVariables|GetStatRef))) (Utilities|Struct|BreakE_SingleStat (LocalVariables|GetStatRef)) 9999999.0)))
    (:NewEnumerator3
      (Development|PrintString "Warning: Set Stat - 
Error: Can not set Total")
      (return)))
  (Stats|Setters|SetStatMember Stat (LocalVariables|GetStatRef))
  (return))

(fn SetStatMember
  (params (Stat :type E_StatList%20Enum :default "NewEnumerator0") (SingleStat :type E%20Single%20Stat%20Structure))
  (bind (_attributevalue _attributeindex _statvalue _statindex) (Stats|Getters|GetStatRef Stat))
  (bind _attributes (Variables|Default|GetAttributes))
  (bind _attributes_2 (Utilities|Struct|BreakE_Attributes _attributes))
  (LocalVariables|SetStatIndex _attributeindex)
  (bind _output_get (LocalVariables|SetStatArray (Utilities|Struct|BreakE_SingleAttribute _attributevalue)))
  (Utilities|Array|SetArrayElem _output_get _statindex SingleStat)
  (bind _structout (Utilities|Struct|SetmembersinE_SingleAttribute (Utilities|Array|Get(acopy) _attributes_2 (LocalVariables|GetStatIndex)) (LocalVariables|GetStatArray)))
  (Utilities|Array|SetArrayElem _attributes_2 (LocalVariables|GetStatIndex) _structout)
  (return))

(fn OperateTotalStat
  (params (Operation :type E_Operators%20Enum :default "NewEnumerator0") (Stat :type E_StatList%20Enum :default "NewEnumerator0") (Value :type Float%20%28double-precision%29))
  (switch Utilities|FlowControl|Switch|SwitchonE_Operators Operation
    (:NewEnumerator0
      (Stats|Functions|ModifyStat "NewEnumerator0" "NewEnumerator1" Stat Value)
      (return))
    (:NewEnumerator1
      (if (>= (- (Stats|Getters|GetStatValue "NewEnumerator2" Stat) Value) 0.0)
        (Stats|Functions|ModifyStat "NewEnumerator1" "NewEnumerator2" Stat Value)
        (return)
        (else
          (bind _output_get (LocalVariables|SetStoredValue (Stats|Getters|GetStatValue "NewEnumerator2" Stat)))
          (Stats|Functions|ModifyStat "NewEnumerator1" "NewEnumerator2" Stat _output_get)
          (Stats|Functions|ModifyStat "NewEnumerator1" "NewEnumerator1" Stat (- Value (LocalVariables|GetStoredValue)))
          (return))))
    (:NewEnumerator2
      (Development|PrintString "Warning: Operate Total Set 
Unable to Set \"Total\" Value")
      (return))))

(fn ScalingStats
  (params (Type :type E_StatType%20Enum :default "NewEnumerator0") (Operation :type E_Operators%20Enum :default "NewEnumerator0") (Attribute :type E%20Single%20Attribute%20Structure) (Value :type Float%20%28double-precision%29))
  (for _array_element (Utilities|Struct|BreakE_SingleAttribute Attribute)
    (LocalVariables|SetStatLocal (.Name (Utilities|Struct|BreakE_SingleStat _array_element)))
    (Stats|Setters|SetStat Type (LocalVariables|GetStatLocal) (Math|Float|Clamp(Float) (Utilities|Select :Index Operation :NewEnumerator0 (+ (Utilities|Select :Index Type :NewEnumerator0 0.0 :NewEnumerator1 (.Default (Utilities|Struct|BreakE_SingleStat _array_element)) :NewEnumerator2 (.Bonus (Utilities|Struct|BreakE_SingleStat _array_element)) :NewEnumerator3 0.0) (* (.Scale (Utilities|Struct|BreakE_SingleStat _array_element)) Value)) :NewEnumerator1 (- (Utilities|Select :Index Type :NewEnumerator0 0.0 :NewEnumerator1 (.Default (Utilities|Struct|BreakE_SingleStat _array_element)) :NewEnumerator2 (.Bonus (Utilities|Struct|BreakE_SingleStat _array_element)) :NewEnumerator3 0.0) (* (.Scale (Utilities|Struct|BreakE_SingleStat _array_element)) Value)) :NewEnumerator2 (* (.Scale (Utilities|Struct|BreakE_SingleStat _array_element)) Value)) 0.0 9999999.0))
    (Stats|Functions|ConditionalStats (LocalVariables|GetStatLocal))))

(fn ConditionalStats
  (params (Stat :type E_StatList%20Enum :default "NewEnumerator0"))
  (switch Utilities|FlowControl|Switch|SwitchonE_StatList Stat
    (:NewEnumerator1
      (CallFunction|CheckExp))
    (:NewEnumerator3
      (CallFunction|CheckHealth))
    (:NewEnumerator5
      (CallFunction|CheckRange))
    (:NewEnumerator6
      (CallFunction|CheckProjectileSpeed))))

(fn LevelUp
  (params (Value :type Float%20%28double-precision%29))
  (Default|CallOnLevelUp))

(fn GetHealthPercent
  (return (/ (Stats|Getters|GetStatValue "NewEnumerator3" "NewEnumerator3") (Stats|Getters|GetStatValue "NewEnumerator3" "NewEnumerator2"))))

(fn GetSpreadAngle
  (return (* (- (Stats|Getters|GetStatValue "NewEnumerator3" "NewEnumerator7") 1.0) (Stats|Getters|GetStatValue "NewEnumerator3" "NewEnumerator8"))))